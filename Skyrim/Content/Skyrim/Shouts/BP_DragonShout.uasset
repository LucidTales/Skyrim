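; Moving projectile actor for a Skyrim-style Fus Ro Dah dragon shout, with a Niagara effect oriented along its travel direction.
; Each tick it sweeps forward by Direction times Speed, without delta-time scaling.
; On overlap it sends each actor a single FusRoDahMessage carrying direction and power level, tracking those already hit.
; Timers switch the effect off after a short active period and destroy the actor later.
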(event EventTick
  (params (DeltaSeconds :type Float%20%28single-precision%29))
  (Transformation|SetActorLocation (+ (* (Variables|Default|GetDirection) (Variables|Default|GetSpeed)) (Transformation|GetActorLocation)) true false))

(event Collision|EventActorBeginOverlap
  (params (OtherActor :type Actor%20Object%20Reference))
  (if (not (Utilities|Set|Contains (Variables|Default|GetOverlappedActors) OtherActor))
    (Utilities|Set|Add (Variables|Default|GetOverlappedActors) OtherActor)
    (Class|BPIShouts|FusRoDah(Message) OtherActor (Variables|Default|GetDirection) (Variables|Default|GetPowerLevel))))

(event EventBeginPlay
  (Utilities|Time|SetTimerbyFunctionName 0 "Deactivate" 2.0)
  (Class|NiagaraComponent|SetVariableQuat (Variables|Default|GetNiagara) "Orientation" (Class|KismetMathLibrary|ToQuaterion(Vector) (Variables|Default|GetDirection))))

(fn ConstructionScript)

(fn Deactivate
  (Components|Activation|Deactivate (Variables|Default|GetNiagara))
  (Utilities|Time|SetTimerbyFunctionName 0 "DestroySelf" 3e+01))

(fn DestroySelf
  (Actor|DestroyActor))