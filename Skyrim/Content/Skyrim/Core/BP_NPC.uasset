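; Skyrim-style NPC that looks at a nearby player and reacts to the Fus Ro Dah shout by power level.
; Weak shouts play a montage and disable movement; the strongest launches it as a ragdoll.
; While ragdolled, the capsule follows the pelvis via ground traces, until a timer triggers a snapshot-based get-up and return to routine.
; An editor spline generates destination points and is destroyed at BeginPlay.
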(event OnComponentBeginOverlap(PlayerDetection)
  (params (OverlappedComponent :type Primitive%20Component%20Object%20Reference) (OtherActor :type Actor%20Object%20Reference) (OtherComp :type Primitive%20Component%20Object%20Reference) (OtherBodyIndex :type Integer) (bFromSweep :type Boolean) (SweepResult :type Hit%20Result%20Structure%20%28by%20ref%29))
  (bind _asbp_skyrim_character (Utilities|Casting|CastToBP_SkyrimCharacter OtherActor))
  (bind _output_get (Variables|Default|SetPlayerCharacter _asbp_skyrim_character))
  (Default|StartLookingat (Variables|Default|GetAnimBP) _output_get))

(event OnComponentEndOverlap(PlayerDetection)
  (params (OverlappedComponent :type Primitive%20Component%20Object%20Reference) (OtherActor :type Actor%20Object%20Reference) (OtherComp :type Primitive%20Component%20Object%20Reference) (OtherBodyIndex :type Integer))
  (if (== OtherActor (Variables|Default|GetPlayerCharacter))
    (Variables|Default|SetPlayerCharacter 0)
    (Default|StopLookingat (Variables|Default|GetAnimBP))))

(event Custom|GetUp
  (Variables|Default|SetbThrown false)
  (Default|SaveSnapshot (Variables|Default|GetAnimBP))
  (Physics|SetSimulatePhysics (Variables|Character|GetMesh) false)
  (Collision|SetCollisionEnabled (Variables|Collision|GetCapsuleComponent) "QueryAndPhysics")
  (Transformation|AttachComponentToComponent (Variables|Character|GetMesh) (Variables|Collision|GetCapsuleComponent) "None" "KeepWorld" "SnapToTarget" "KeepRelative" false)
  (Transformation|SetRelativeLocation (Variables|Character|GetMesh) (Variables|Default|GetInitialRelativeLocation) false false)
  (Utilities|FlowControl|Delay 0.1)
  (Default|GetUp (Variables|Default|GetAnimBP))
  (Default|GoBacktoRoutine (Variables|Default|GetNPCController)))

(event EventBeginPlay
  (bind _asabp_character (Utilities|Casting|CastToABP_Character (Components|SkeletalMesh|GetAnimInstance (Variables|Character|GetMesh))))
  (Variables|Default|SetAnimBP _asabp_character)
  (Variables|Default|SetInitialRelativeLocation (Variables|/Script/Engine.SceneComponent|GetRelativeLocation (Variables|Character|GetMesh)))
  (Components|DestroyComponent (Variables|Default|GetSpline)))

(event EventTick
  (params (DeltaSeconds :type Float%20%28single-precision%29))
  (CallFunction|GetUpCheck))

(event EventFusRoDah
  (params (Direction :type Vector :default "0, 0, 0") (PowerLevel :type Integer))
  (CallFunction|ReceiveFusRohDah Direction PowerLevel))

(fn ConstructionScript
  (Utilities|Array|Clear (Variables|Default|GetDestinations))
  (for _index (range 0 (- (Spline|GetNumberOfSplinePoints (Variables|Default|GetSpline)) 1))
    (bind _returnvalue (AddComponent|AddStaticMeshComponent false (Math|Transform|MakeTransform (Spline|GetLocationatSplinePoint (Variables|Default|GetSpline) _index "Local") "0, 0, 0" (Math|Conversions|ToVector(Float) 0.5))))
    (Utilities|Array|Add (Variables|Default|GetDestinations) (Transformation|GetWorldLocation _returnvalue))))

(fn GetUpCheck
  (if (Variables|Default|GetbGetUpCheck)
    (CallFunction|GetUp)
    (Variables|Default|SetbGetUpCheck false)
    (else
      (CallFunction|MoveCapsule))))

(fn MoveCapsule
  (bind _mesh (Variables|Character|GetMesh))
  (bind _returnvalue (Transformation|GetSocketLocation _mesh "pelvis"))
  (if (Variables|Default|GetbThrown)
    (bind (_outhit _returnvalue_2) (Collision|LineTraceByChannel _returnvalue (+ _returnvalue (* (Transformation|GetActorUpVector) -2e+02)) "TraceTypeQuery1" false 0 "None"))
    (if _returnvalue_2
      (Variables|Default|SetCapsuleLocation (+ (.impactpoint _outhit) (Math|Vector|MakeVector 0.0 0.0 (Components|Capsule|GetScaledCapsuleHalfHeight (Variables|Collision|GetCapsuleComponent)))))
      (Transformation|SetWorldLocation (Variables|Collision|GetCapsuleComponent) (Variables|Default|GetCapsuleLocation) false false)
      (Transformation|SetWorldRotation (Variables|Collision|GetCapsuleComponent) (Math|Rotator|MakeRotator 0.0 0.0 (.yaw (Math|Rotator|MakeRotfromX (Class|KismetAnimationLibrary|DirectionBetweenSockets (Variables|Character|GetMesh) "neck_01" "pelvis")))) false false))))

(fn StartGetUp
  (Variables|Default|SetbGetUpCheck true))

(fn ReceiveFusRohDah
  (params (Direction :type Vector) (PowerLevel :type Integer))
  (switch int PowerLevel
    (:0
      (Animation|PlayAnimMontage "/Game/Skyrim/Characters/Animations/AM_FusReaction.AM_FusReaction" 3.0 "None")
      (Pawn|Components|CharacterMovement|DisableMovement (Variables|Character|GetCharacterMovement) :!label _label))
    (:1
      (Animation|PlayAnimMontage "/Game/Skyrim/Characters/Animations/AM_FusReaction.AM_FusReaction" 2.0 "None")
      (goto _label))
    (:2
      (Pawn|Components|CharacterMovement|DisableMovement (Variables|Character|GetCharacterMovement))
      (Physics|SetSimulatePhysics (Variables|Character|GetMesh) true)
      (Collision|SetCollisionEnabled (Variables|Character|GetMesh) "QueryAndPhysics")
      (Collision|SetCollisionEnabled (Variables|Collision|GetCapsuleComponent) "NoCollision")
      (Physics|AddImpulse (Variables|Character|GetMesh) (* Direction (Variables|Default|GetThrowForce)) "pelvis" true)
      (Variables|Default|SetbThrown true)
      (Utilities|Time|SetTimerbyFunctionName 0 "StartGetUp" 2.0))))