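; AI controller that walks a BP_NPC along a looping patrol route built from the pawn's Destinations list.
; On BeginPlay it registers itself on the pawn, caches the destinations and moves to the first one.
; Tick checks the pawn's distance to the active destination and advances to the next on arrival, wrapping to the start.
; GoBackToRoutine re-issues the move to the current destination so an interrupted route can resume.
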(event EventTick
  (params (DeltaSeconds :type Float%20%28single-precision%29))
  (CallFunction|CheckifatDestination))

(event EventBeginPlay
  (bind _asbp_npc (Utilities|Casting|CastToBP_NPC (Pawn|GetControlledPawn)))
  (bind _output_get (Variables|Default|SetControlledPawn _asbp_npc))
  (Variables|/Game/Skyrim/Core/BP_NPC.BP_NPC_C|SetNPCController _output_get self)
  (Variables|Default|SetPawnDestinations (Variables|/Game/Skyrim/Core/BP_NPC.BP_NPC_C|GetDestinations _output_get))
  (Variables|Default|SetDestinationMaxIndex (- (Utilities|Array|Length (Variables|/Game/Skyrim/Core/BP_NPC.BP_NPC_C|GetDestinations _output_get)) 1))
  (AI|Navigation|MovetoLocation (Utilities|Array|Get(acopy) (Variables|Default|GetPawnDestinations)) -1.0 true true false true 0))

(fn ConstructionScript)

(fn MovetoNextDestination
  (if (== (Variables|Default|GetActiveDestination) (Variables|Default|GetDestinationMaxIndex))
    (Variables|Default|SetActiveDestination 0)
    (else
      (Variables|Default|SetActiveDestination (+ (Variables|Default|GetActiveDestination) 1))))
  (AI|Navigation|MovetoLocation (Utilities|Array|Get(acopy) (Variables|Default|GetPawnDestinations) (Variables|Default|GetActiveDestination)) -1.0 true true false true 0))

(fn CheckifatDestination
  (if (Math|Vector|Equal(Vector) (Transformation|GetActorLocation (Variables|Default|GetControlledPawn)) (Utilities|Array|Get(acopy) (Variables|Default|GetPawnDestinations) (Variables|Default|GetActiveDestination)) 5e+01)
    (CallFunction|MovetoNextDestination)))

(fn GoBacktoRoutine
  (AI|Navigation|MovetoLocation (Utilities|Array|Get(acopy) (Variables|Default|GetPawnDestinations) (Variables|Default|GetActiveDestination)) -1.0 true true false true 0))